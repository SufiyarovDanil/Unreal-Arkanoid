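; Brick actor that reacts to Ball overlaps and can take one or two hits before it is destroyed.
; On BeginPlay it moves its Cube to a fixed world height, keeping X and Y.
; When a Ball overlaps its Box, a set SecondHit flag is cleared and the Cube switches to the BallRed material; otherwise the brick destroys itself after a short delay.
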(event `self.ReceiveBeginPlay`
  (bind _cube (`self.Cube`))
  (bind (_returnvalue_x _returnvalue_y) (`KismetMathLibrary.BreakVector` (`SceneComponent.K2_GetComponentLocation` _cube)))
  (`SceneComponent.K2_SetWorldLocation` _cube (`KismetMathLibrary.MakeVector` _returnvalue_x _returnvalue_y 100.0) false false))

(event `self.Box.OnComponentBeginOverlap`
  (params (OverlappedComponent :type "PrimitiveComponent Object Reference") (OtherActor :type "Actor Object Reference") (OtherComp :type "PrimitiveComponent Object Reference") (OtherBodyIndex :type Integer) (bFromSweep :type Boolean) (SweepResult :type "HitResult Structure (by ref)"))
  (cast `/Game/Blueprints/Ball` OtherActor)
  (if (`self.SecondHit`)
    (`PrimitiveComponent.SetMaterial` (`self.Cube`) 0 "/Game/Materials/BallRed.BallRed")
    (set `self.SecondHit` false)
    (else
      (`KismetSystemLibrary.Delay` 0.1)
      (`self.K2_DestroyActor`))))

(fn `UserConstructionScript`)