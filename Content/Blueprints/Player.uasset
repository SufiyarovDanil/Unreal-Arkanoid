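; Player paddle Blueprint for a touch-controlled brick-breaker that also handles level completion and failure.
; While touched, Tick moves the Player component along X to the Visibility trace hit under the finger, keeping Y and using a fixed height.
; BeginPlay polls for remaining Brick actors on a delay loop and opens the hard-coded Level2 when none remain.
; A Ball overlapping RestartTrigger reloads the current level after a short delay.
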(event `self.ReceiveBeginPlay`
  (bind _outactors (`GameplayStatics.GetAllActorsOfClass` "/Game/Blueprints/Brick.Brick_C" :!label _label))
  (if (== (`KismetArrayLibrary.Array_Length` _outactors) 0)
    (`GameplayStatics.OpenLevel` "Level2")
    (else
      (`KismetSystemLibrary.Delay` 3.0)
      (goto _label))))

(event `InputTouch`
  (params (Location :type "Vector Structure") (FingerIndex :type "ETouchIndex Enum"))
  (:`Pressed`
    (set `self.isTouched` true))
  (:`Released`
    (set `self.isTouched` false)))

(event `self.ReceiveTick`
  (params (DeltaSeconds :type "Float (single-precision)"))
  (bind _player (`self.Player`))
  (bind _player_2 (`self.Player`))
  (bind (_returnvalue_x _returnvalue_y) (`KismetMathLibrary.BreakVector` (`SceneComponent.K2_GetComponentLocation` _player)))
  (if (`self.isTouched`)
    (`SceneComponent.K2_SetWorldLocation` _player (`KismetMathLibrary.MakeVector` (.x (`.Location` (`GameplayStatics.BreakHitResult` (`PlayerController.GetHitResultUnderFingerByChannel` (`GameplayStatics.GetPlayerController` 0) "Touch1" "TraceTypeQuery1" true)))) _returnvalue_y 100.0) false false)
    (else
      (`SceneComponent.K2_SetWorldLocation` _player_2 (`SceneComponent.K2_GetComponentLocation` _player_2) false false))))

(event `self.RestartTrigger.OnComponentBeginOverlap`
  (params (OverlappedComponent :type "PrimitiveComponent Object Reference") (OtherActor :type "Actor Object Reference") (OtherComp :type "PrimitiveComponent Object Reference") (OtherBodyIndex :type Integer) (bFromSweep :type Boolean) (SweepResult :type "HitResult Structure (by ref)"))
  (cast `/Game/Blueprints/Ball` OtherActor)
  (`KismetSystemLibrary.Delay` 0.5)
  (bind _returnvalue (`GameplayStatics.GetCurrentLevelName` true))
  (`GameplayStatics.OpenLevel` (`KismetStringLibrary.Conv_StringToName` _returnvalue)))

(fn `UserConstructionScript`)